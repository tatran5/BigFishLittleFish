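; BP_Corrosive is a world object that reacts to whether the player's fish is the Acid type.
; Each tick it casts the player character to BP_Fish and reads FishType.
; PlatformBoxCollider is shown in game for Acid and hidden for any other type.
; The graph toggles only that component's hidden flag and does not change its collision settings.
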(event `self.ReceiveTick`
  (params (DeltaSeconds :type "Float (single-precision)"))
  (bind _returnvalue (`GameplayStatics.GetPlayerCharacter` 0))
  (bind _platformboxcollider (`self.PlatformBoxCollider`))
  (`parent.ReceiveTick` DeltaSeconds)
  (if (`KismetSystemLibrary.IsValid` _returnvalue)
    (bind _asbp_fish (cast `/Game/Blueprints/Fish/BP_Fish` _returnvalue))
    (if (== (`/Game/Blueprints/Fish/BP_Fish.FishType` _asbp_fish) "Acid")
      (`SceneComponent.SetHiddenInGame` _platformboxcollider false false)
      (else
        (`SceneComponent.SetHiddenInGame` _platformboxcollider true false)))))

(fn `UserConstructionScript`
  (`parent.UserConstructionScript`))