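; BP_Poison is a hazard object that costs a life when a player-controlled fish touches it.
; Each Tick, it runs a box overlap at the trigger mesh's location, sized by its Box component and filtered to one object type.
; For each non-AI BP_Fish found, it decreases lives on the BP_Global actor cached at BeginPlay and plays the fish's lose-life animation, with no cooldown here.
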(event `self.ReceiveBeginPlay`
  (bind _returnvalue (`GameplayStatics.GetActorOfClass` "/Game/BluePrints/GameState/BP_Global.BP_Global_C")))

(event `self.ReceiveTick`
  (params (DeltaSeconds :type "Float (single-precision)"))
  (bind _outactors (`KismetSystemLibrary.BoxOverlapActors` (`SceneComponent.K2_GetComponentLocation` (`self.TriggerMesh`)) (`BoxComponent.GetScaledBoxExtent` (`self.Box`)) (`|MakeArray` "ObjectTypeQuery8" :!type "EObjectTypeQuery Enum")))
  (for _array_element _outactors
    (bind _asbp_fish (cast `/Game/BluePrints/Fish/BP_Fish` _array_element))
    (if (not (`/Game/BluePrints/Fish/BP_Fish.IsAI` _asbp_fish))
      (`/Game/BluePrints/GameState/BP_Global.DecreaseLives` (stale `self.ReceiveBeginPlay` _returnvalue))
      (`/Game/BluePrints/Fish/BP_Fish.AnimateLoseLife` _asbp_fish))))

(fn `UserConstructionScript`)