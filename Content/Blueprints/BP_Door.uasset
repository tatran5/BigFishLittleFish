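; BP_Door is a sliding door actor that rises vertically while its Opening flag is true.
; The construction script clears Opening and stores the start location as InitialPos.
; Tick lifts it by a fixed, frame-rate-dependent step with sweep, capped at Range above InitialPos.
; When Opening is false, the downward step is clamped to a minimum of current Z, so the door does not descend.
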(event `self.ReceiveTick`
  (params (DeltaSeconds :type "Float (single-precision)"))
  (bind _z (.z (`self.K2_GetActorLocation`)))
  (bind _x (.x (`self.initialPos`)))
  (bind _y (.y (`self.initialPos`)))
  (bind _z_2 (.z (`self.initialPos`)))
  (bind _returnvalue (+ _z_2 (`self.range`)))
  (`parent.ReceiveTick` DeltaSeconds)
  (if (`self.opening`)
    (`self.K2_SetActorLocation` (`KismetMathLibrary.MakeVector` _x _y (`KismetMathLibrary.FClamp` (+ _z 25.0) _z_2 _returnvalue)) true)
    (else
      (`self.K2_SetActorLocation` (`KismetMathLibrary.MakeVector` _x _y (`KismetMathLibrary.FClamp` (- _z 25.0) _z _returnvalue)) true))))

(fn `UserConstructionScript`
  (`parent.UserConstructionScript`)
  (set `self.opening` false)
  (set `self.initialPos` (`self.K2_GetActorLocation`)))