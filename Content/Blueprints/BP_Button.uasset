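; BP_Button is a pressure-plate button actor that controls a connected door.
; Each tick it runs a box overlap query matching its platform collider's location and scaled extent, filtered to a single object type.
; The boolean result is written straight to the connected door's Opening flag, so that flag is true only while a matching object is in the box.
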(event `self.ReceiveTick`
  (params (DeltaSeconds :type "Float (single-precision)"))
  (bind _platformboxcollider (`self.PlatformBoxCollider`))
  ;[1 1 1] Detect Being Pressed
  (`parent.ReceiveTick` DeltaSeconds)
  (bind (_outactors _returnvalue) (`KismetSystemLibrary.BoxOverlapActors` (`SceneComponent.K2_GetComponentLocation` _platformboxcollider) (`BoxComponent.GetScaledBoxExtent` _platformboxcollider) (`|MakeArray` "ObjectTypeQuery9" :!type "EObjectTypeQuery Enum")))
  (set `/Game/Blueprints/BP_Door.opening` _returnvalue (`self.connectedDoor`)))

(fn `UserConstructionScript`
  (`parent.UserConstructionScript`))