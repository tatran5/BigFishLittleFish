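; BP_PlayerAcidFish is a player fish Blueprint in the Test folder whose ability fires acid projectiles.
; Pressing the Ability input spawns a BP_AcidProjectile just beside the actor along the Y axis.
; The FacingRight boolean is converted to a sign that sets both the offset direction and the projectile's yaw, so shots follow the facing.
; Spawning nudges clear of collisions or is skipped if blocked.
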(event `InputAction|Ability`
  (params (Key :type "Key Structure"))
  (bind _returnvalue (- (* (`KismetMathLibrary.Conv_BoolToDouble` (`self.facingRight`)) 2.0) 1.0))
  (:`Pressed`
    (`|SpawnActorFromClass` "/Game/Blueprints/Objects/BP_AcidProjectile.BP_AcidProjectile_C" (`KismetMathLibrary.MakeTransform` (+ (`self.K2_GetActorLocation`) (`KismetMathLibrary.MakeVector` 0.0 _returnvalue)) (`KismetMathLibrary.RotatorFromAxisAndAngle` (0.0 0.0 1.0) (* _returnvalue 90.0))) "AdjustIfPossibleButDontSpawnIfColliding" "OverrideRootScale" null null)))

(fn `UserConstructionScript`
  (`parent.UserConstructionScript`))