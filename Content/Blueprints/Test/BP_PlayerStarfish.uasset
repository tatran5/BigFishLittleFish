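; Test player starfish that moves along the Y-Z plane and can break off up to two BP_StarfishLeg actors.
; The Ability input spawns a leg offset toward the facing direction.
; Swept location offsets drive horizontal and upward-only vertical movement, with horizontal input also moving every leg in the world.
; Each Tick, an overlap query at TriggerCapsule destroys touched legs and decrements ActiveLegs, so they can be spawned again.
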(event `InputAction|Ability`
  (params (Key :type "Key Structure"))
  ;[1 1 1] Ability: Break off legs
  (:`Pressed`
    (if (< (`self.activeLegs`) 2)
      (`|SpawnActorFromClass` "/Game/Blueprints/Fish/BP_StarfishLeg.BP_StarfishLeg_C" (`KismetMathLibrary.MakeTransform` (+ (`self.K2_GetActorLocation`) (`KismetMathLibrary.MakeVector` 0.0 (* (- (* (`KismetMathLibrary.Conv_BoolToDouble` (`self.facingRight`)) 2.0) 1.0) 3.0) 2.0))) "AdjustIfPossibleButAlwaysSpawn" "OverrideRootScale" null null)
      (set `self.activeLegs` (+ (`self.activeLegs`) 1)))))

(event `InputAxis|MoveVertical`
  (params (AxisValue :type "Float (single-precision)"))
  ;[1 1 1] Movement (modified for Starfish specifically)
  (if (> AxisValue 0.0)
    (`PrimitiveComponent.SetPhysicsAngularVelocityInDegrees` (`self.CapsuleComponent`) (0.0 0.0 0.0) false "None")
    (`self.K2_SetActorLocation` (+ (`self.K2_GetActorLocation`) (`KismetMathLibrary.MakeVector` 0.0 0.0 (* AxisValue 5.0))) true)))

(event `InputAxis|MoveHorizontal`
  (params (AxisValue :type "Float (single-precision)"))
  ;[1 1 1] Movement (modified for Starfish specifically)
  (set `self.facingRight` (> AxisValue 0.0))
  (`self.K2_SetActorLocation` (+ (`self.K2_GetActorLocation`) (`KismetMathLibrary.MakeVector` 0.0 (* AxisValue 3.0))) true)
  (bind _outactors (`GameplayStatics.GetAllActorsOfClass` "/Game/Blueprints/Fish/BP_StarfishLeg.BP_StarfishLeg_C"))
  (for _array_element _outactors
    (`PrimitiveComponent.SetPhysicsAngularVelocityInDegrees` (`/Game/Blueprints/Fish/BP_StarfishLeg.LegCollider` _array_element) (0.0 0.0 0.0) false "None")
    (`self.K2_SetActorLocation` _array_element (+ (`self.K2_GetActorLocation` _array_element) (`KismetMathLibrary.MakeVector` 0.0 (* AxisValue 3.0))) true false)))

(event `self.ReceiveTick`
  (params (DeltaSeconds :type "Float (single-precision)"))
  (bind _triggercapsule (`self.TriggerCapsule`))
  ;[1 1 1] Leg Collision (absorb leg)
  (`parent.ReceiveTick` DeltaSeconds)
  (bind (_outactors _returnvalue) (`KismetSystemLibrary.CapsuleOverlapActors` (`SceneComponent.K2_GetComponentLocation` _triggercapsule) (`CapsuleComponent.CapsuleRadius` _triggercapsule) (`CapsuleComponent.GetScaledCapsuleHalfHeight` _triggercapsule) (`|MakeArray` "ObjectTypeQuery9" :!type "EObjectTypeQuery Enum") "/Game/Blueprints/Fish/BP_StarfishLeg.BP_StarfishLeg_C" (`|MakeArray` (`GameplayStatics.GetPlayerCharacter` 0) :!type "Actor Object Reference")))
  (if _returnvalue
    (for _array_element _outactors
      (`self.K2_DestroyActor` _array_element)
      (set `self.activeLegs` (- (`self.activeLegs`) 1)))))

(fn `UserConstructionScript`
  (`parent.UserConstructionScript`)
  (`PrimitiveComponent.SetCollisionObjectType` (`self.TriggerCapsule`) "ECC_GameTraceChannel3"))