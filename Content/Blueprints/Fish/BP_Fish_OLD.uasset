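; Fish pawn, serving as both player and AI, for a side-view game of swallowing smaller fish.
; Player input drives drag-damped Y/Z movement; AI chases, flees or wanders by player distance and relative scale.
; Player overlaps either swallow smaller fish into BP_Global's inventory or cost a life and reset position.
; Swallow and Spit change form by destroying the pawn and possessing a new subclass; Spit also releases the current type as AI.
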(event `InputAction|Pause` :paused true
  (params (Key :type "Key Structure"))
  ;[1 1 1] Pause
  (:`Pressed`
    (`/Engine/EditorBlueprintResources/StandardMacros.FlipFlop`
      (:`A`
        (`GameplayStatics.SetGamePaused` true)
        (`Widget.SetVisibility` (stale `self.ReceiveBeginPlay` _returnvalue) "Visible"))
      (:`B`
        (`GameplayStatics.SetGamePaused` false)
        (`Widget.SetVisibility` (stale `self.ReceiveBeginPlay` _returnvalue) "Hidden")))))

(event `self.ReceiveBeginPlay`
  (bind _returnvalue (`|CreateWidget` "/Game/Blueprints/UI/Gameplay/UI_Pause.UI_Pause_C"))
  (`UserWidget.AddToViewport` _returnvalue 0)
  (`Widget.SetVisibility` _returnvalue "Hidden")
  (`PrimitiveComponent.SetCollisionObjectType` (`self.TriggerCapsule`) "ECC_GameTraceChannel2")
  (set `self.VyMax` 5.0)
  (set `self.VzMax` 5.0)
  (set `self.drag_z` 0.1)
  (set `self.drag_y` 0.1)
  (set `self.delta_v` 0.4))

(event `self.ReceiveTick`
  (params (DeltaSeconds :type "Float (single-precision)"))
  (bind _injurytimer (`self.InjuryTimer`))
  (if (`self.FacingRight`)
    (`SceneComponent.K2_SetRelativeRotation` :`self` (`self.Mesh`) :`bSweep` true)
    (else
      (`SceneComponent.K2_SetRelativeRotation` (`self.Mesh`) (struct :`Yaw` 180.0) true false)))
  (if (`self.IsAI`)
    (`self.Handle AI` (`self.DistanceOfDetection`))
    (else
      ;[1 1 1] Drag (Z)
      (if (< (`self.Vz`) 0.0)
        (set `self.drag_z` (`KismetMathLibrary.Abs` (`self.drag_z`)))
        (bind _output_get (set `self.Vz` (+ (`self.Vz`) (`self.drag_z`))))
        (if (> _output_get 0.0)
          (set `self.Vz` 0.0))
        (else
          ;[1 1 1] Movement/Action
          (if (> (`self.drag_z`) 0.0)
            (set `self.drag_z` (* (`self.drag_z`) -1.0)))
          (bind _output_get_2 (set `self.Vz` (+ (`self.Vz`) (`self.drag_z`))))
          (if (< _output_get_2 0.0)
            ;[1 1 1] Update Player Z
            (set `self.Vz` 0.0))))
      (`self.K2_SetActorLocation` (+ (`self.K2_GetActorLocation`) (`KismetMathLibrary.MakeVector` 0.0 0.0 (`self.Vz`))) true)
      ;[1 1 1] Update Player Y
      (if (< (`self.Vy`) 0.0)
        (set `self.drag_y` (`KismetMathLibrary.Abs` (`self.drag_y`)))
        (bind _output_get_3 (set `self.Vy` (+ (`self.Vy`) (`self.drag_y`))))
        (if (> _output_get_3 0.0)
          (set `self.Vy` 0.0))
        (else
          (if (> (`self.drag_y`) 0.0)
            (set `self.drag_y` (* (`self.drag_y`) -1.0)))
          (bind _output_get_4 (set `self.Vy` (+ (`self.Vy`) (`self.drag_y`))))
          (if (< _output_get_4 0.0)
            (set `self.Vy` 0.0))))
      (`self.K2_SetActorLocation` (+ (`self.K2_GetActorLocation`) (`KismetMathLibrary.MakeVector` 0.0 (`self.Vy`))) true)
      ;[1 1 1] Hurt Animation
      (if (< _injurytimer 100)
        (bind _output_get_5 (set `self.InjuryTimer` (+ _injurytimer 1)))
        (`SceneComponent.SetVisibility` (`self.Mesh`) (`KismetMathLibrary.Conv_IntToBool` (`KismetMathLibrary.Round` (+ (/ (`KismetMathLibrary.DegSin` (* (`KismetMathLibrary.Conv_IntToDouble` _output_get_5) 18.0)) 2.0) 0.5))) true)
        (else
          (`SceneComponent.SetVisibility` (`self.Mesh`) true true))))))

(event `InputAction|Spit`
  (params (Key :type "Key Structure"))
  ;[1 1 1] Movement/Action
  (:`Pressed`
    (`self.Spit`)))

(event `InputAxis|MoveVertical`
  (params (AxisValue :type "Float (single-precision)"))
  (bind _returnvalue (* (`self.VzMax`) -1.0))
  ;[1 1 1] Physics Z Movement
  (if (> AxisValue 0.0)
    (bind _output_get (set `self.Vz` (+ (`self.Vz`) (`self.delta_v`))))
    (if (> _output_get (`self.VzMax`))
      (set `self.Vz` (`self.VzMax`)))
    (elif (not (== AxisValue 0.0))
      (bind _output_get_2 (set `self.Vz` (- (`self.Vz`) (`self.delta_v`))))
      (if (< _output_get_2 _returnvalue)
        (set `self.Vz` _returnvalue)))))

(event `self.ReceiveActorBeginOverlap`
  (params (OtherActor :type "Actor Object Reference"))
  (`self.HandlePlayerCollision`))

(event `InputAxis|MoveHorizontal`
  (params (AxisValue :type "Float (single-precision)"))
  (bind _returnvalue (* (`self.VyMax`) -1.0))
  ;[1 1 1] Physics Y Movement
  (if (> AxisValue 0.0)
    (bind _output_get (set `self.Vy` (+ (`self.Vy`) (`self.delta_v`))))
    (if (> _output_get (`self.VyMax`))
      (set `self.Vy` (`self.VyMax`)))
    (if (> AxisValue 0.0) :!label _label
      (set `self.facingRight` true)
      (elif (< AxisValue 0.0)
        (set `self.facingRight` false)
        (elif (< (`self.Vy`) 0.0)
          (set `self.facingRight` false)
          (else
            (set `self.facingRight` true)))))
    (elif (not (== AxisValue 0.0))
      (bind _output_get_2 (set `self.Vy` (- (`self.Vy`) (`self.delta_v`))))
      (if (< _output_get_2 _returnvalue)
        (set `self.Vy` _returnvalue)
        (goto _label)
        (else
          (goto _label))))))

(fn `Animate Lose Life`
  (if (== (`self.InjuryTimer`) 100)
    (set `self.InjuryTimer` 0)))

(fn `GetIndexFirstEmptyElement`
  (params (Inventory :type "Array of Name"))
  (returns (EmptyIndex :type Integer))
  ;[1 1 1] Find and return the index of the first empty element in the array. If there is no empty index, return -1
  (for (_array_element _array_index) Inventory
    (if (== _array_element "None")
      (return _array_index)))
  (return -1))

(fn `GetInventory`
  (returns (Inventory :type "Array of Name"))
  (bind _outactors (`GameplayStatics.GetAllActorsOfClass` "/Game/Blueprints/GameState/BP_Global.BP_Global_C"))
  ;[1 1 1] There should only be one element in the array
  (for _array_element _outactors
    (return (`/Game/Blueprints/GameState/BP_Global.Inventory` _array_element))))

(fn `GetSelfToPlayer`
  (returns (SelfToPlayer :type "Vector Structure"))
  (return (- (`self.K2_GetActorLocation` (`GameplayStatics.GetPlayerCharacter` 0)) (`self.K2_GetActorLocation`))))

(fn `Handle AI`
  (params (DistanceOfDetection :type "Float (double-precision)"))
  (locals (SelfToPlayer :type "Vector Structure") (PlayerAsFish :type "/Game/Blueprints/Fish/BP_Fish_OLD Object Reference"))
  (bind _selftoplayer (`self.GetSelfToPlayer`))
  (bind _output_get (set `local.SelfToPlayer` _selftoplayer))
  (bind _seeplayer (`self.SeePlayer` _output_get))
  (if _seeplayer
    (bind _asbp_fish (cast `/Game/Blueprints/Fish/BP_Fish_OLD` (`GameplayStatics.GetPlayerCharacter` 0)))
    (bind _output_get_2 (set `local.PlayerAsFish` _asbp_fish))
    (bind _selfislarger (`self.SelfIsLarger` _output_get_2))
    (if _selfislarger
      (`self.RunToPlayer` (`local.SelfToPlayer`))
      (else
        (bind _selfissmaller (`self.SelfIsSmaller` (`local.PlayerAsFish`)))
        (if _selfissmaller
          (`self.RunFromPlayer` (`local.SelfToPlayer`))
          (else
            (`self.Wander`)))))
    (else
      (`self.Wander`))))

(fn `HandlePlayerCollision`
  (locals (Inventory :type "Array of Name"))
  (bind _triggercapsule (`self.TriggerCapsule`))
  (bind _triggercapsule_2 (`self.TriggerCapsule`))
  (bind _returnvalue (`SceneComponent.K2_GetComponentLocation` _triggercapsule))
  (bind _returnvalue_2 (`CapsuleComponent.GetScaledCapsuleHalfHeight` _triggercapsule))
  (bind _capsuleradius (`CapsuleComponent.CapsuleRadius` _triggercapsule))
  (if (not (`self.IsAI`))
    ;[1 1 1] CollisionDetectionFish
    (`KismetSystemLibrary.DrawDebugCapsule` _returnvalue _returnvalue_2 _capsuleradius (struct) (struct :`R` 0.670283 :`G` 1.0 :`B` 0.646556 :`A` 1.0))
    (bind (_outactors _returnvalue_3) (`KismetSystemLibrary.CapsuleOverlapActors` _returnvalue _capsuleradius _returnvalue_2 (`|MakeArray` "ObjectTypeQuery8" :!type "EObjectTypeQuery Enum") null (`|MakeArray` self :!type "Actor Object Reference")))
    (if _returnvalue_3
      (for _array_element _outactors
        (if (< (`KismetMathLibrary.VSize` (`self.GetActorScale3D` _array_element)) (`KismetMathLibrary.VSize` (`self.GetActorScale3D`)))
          (bind _asbp_fish (cast `/Game/Blueprints/Fish/BP_Fish_OLD` _array_element))
          (bind _swallowed (`self.Swallow` _asbp_fish))
          (if _swallowed
            (`self.K2_DestroyActor` _array_element))
          (else
            ;[1 1 1] CollisionDetectionEnemy
            ;;[1 1 1] There is only 1 object in the array. Update lives and UI
            (bind _outactors_2 (`GameplayStatics.GetAllActorsOfClass` "/Game/Blueprints/GameState/BP_Global.BP_Global_C"))
            (for _array_element_2 _outactors_2
              (`/Game/Blueprints/GameState/BP_Global.DecreaseLives` _array_element_2)
              (`self.K2_SetActorLocation` (-170.0 0.0 112.0) false true)))))
      (else
        (bind (_outactors_3 _returnvalue_4) (`KismetSystemLibrary.CapsuleOverlapActors` (`SceneComponent.K2_GetComponentLocation` _triggercapsule_2) (`CapsuleComponent.CapsuleRadius` _triggercapsule_2) (`CapsuleComponent.GetScaledCapsuleHalfHeight` _triggercapsule_2) (`|MakeArray` "ObjectTypeQuery7" :!type "EObjectTypeQuery Enum") null (`|MakeArray` self :!type "Actor Object Reference")))
        (if _returnvalue_4
          _)))))

(fn `RunFromPlayer`
  (params (SelfToPlayer :type "Vector Structure"))
  (set `self.FacingRight` (< (.y SelfToPlayer) 0.0))
  (`self.K2_SetActorLocation` (+ (`self.K2_GetActorLocation`) (* (`KismetMathLibrary.Normal` (* SelfToPlayer -1)) (`self.Speed`)))))

(fn `RunToPlayer`
  (params (SelfToPlayer :type "Vector Structure"))
  (set `self.FacingRight` (> (.y SelfToPlayer) 0.0))
  (`self.K2_SetActorLocation` (+ (`self.K2_GetActorLocation`) (* (`KismetMathLibrary.Normal` SelfToPlayer) (`self.Speed`)))))

(fn `SeePlayer`
  (params (SelfToPlayer :type "Vector Structure"))
  (returns (SeePlayer :type Boolean))
  (return (and (< (`KismetMathLibrary.VSize` SelfToPlayer) (`self.DistanceOfDetection`)) true)))

(fn `SelfIsLarger`
  (params (Fish :type "/Game/Blueprints/Fish/BP_Fish_OLD Object Reference"))
  (returns (SelfIsLarger :type Boolean))
  (return (> (`KismetMathLibrary.VSize` (`self.GetActorScale3D`)) (`KismetMathLibrary.VSize` (`self.GetActorScale3D` Fish)))))

(fn `SelfIsSmaller`
  (params (Fish :type "/Game/Blueprints/Fish/BP_Fish_OLD Object Reference"))
  (returns (SelfIsSmaller :type Boolean))
  (return (< (`KismetMathLibrary.VSize` (`self.GetActorScale3D`)) (`KismetMathLibrary.VSize` (`self.GetActorScale3D` Fish)))))

(fn `SpawnFish`
  (params (FishType :type Name) (Location :type "Vector Structure") (Rotation :type "Rotator Structure"))
  (switch `name` FishType
    (:`Default`
      (bind _returnvalue (`AIBlueprintHelperLibrary.SpawnAIFromClass` "/Game/Blueprints/Fish/BP_FishDefault.BP_FishDefault_C" null (`local.Location`) (`local.Rotation`) :!label _label))
      (bind _asbp_fish (cast `/Game/Blueprints/Fish/BP_Fish_OLD` _returnvalue))
      (set `/Game/Blueprints/Fish/BP_Fish_OLD.IsAI` true _asbp_fish))
    (:`Glow`
      (bind _returnvalue_2 (`AIBlueprintHelperLibrary.SpawnAIFromClass` "/Game/Blueprints/Fish/BP_FishGlow.BP_FishGlow_C" null (`local.Location`) (`local.Rotation`)))
      (bind _asbp_fish_2 (cast `/Game/Blueprints/Fish/BP_Fish_OLD` _returnvalue_2))
      (set `/Game/Blueprints/Fish/BP_Fish_OLD.IsAI` true _asbp_fish_2))
    (:`Tiny`
      (bind _returnvalue_3 (`AIBlueprintHelperLibrary.SpawnAIFromClass` "/Game/Blueprints/Fish/BP_FishTiny.BP_FishTiny_C" null (`local.Location`) (`local.Rotation`)))
      (bind _asbp_fish_3 (cast `/Game/Blueprints/Fish/BP_Fish_OLD` _returnvalue_3))
      (set `/Game/Blueprints/Fish/BP_Fish_OLD.IsAI` true _asbp_fish_3))
    (:`InitialDefault`
      (goto _label))
    (:`Starfish`
      (bind _returnvalue_4 (`AIBlueprintHelperLibrary.SpawnAIFromClass` "/Game/Blueprints/Fish/BP_FishStarfish.BP_FishStarfish_C" null (`local.Location`) (`local.Rotation`)))
      (bind _asbp_fish_4 (cast `/Game/Blueprints/Fish/BP_Fish_OLD` _returnvalue_4))
      (set `/Game/Blueprints/Fish/BP_Fish_OLD.IsAI` true _asbp_fish_4))
    (:`Acid`
      (bind _returnvalue_5 (`AIBlueprintHelperLibrary.SpawnAIFromClass` "/Game/Blueprints/Fish/BP_FishAcid.BP_FishAcid_C" null (`local.Location`) (`local.Rotation`)))
      (bind _asbp_fish_5 (cast `/Game/Blueprints/Fish/BP_Fish_OLD` _returnvalue_5))
      (set `/Game/Blueprints/Fish/BP_Fish_OLD.IsAI` true _asbp_fish_5))
    (:`Bubble`
      (bind _returnvalue_6 (`AIBlueprintHelperLibrary.SpawnAIFromClass` "/Game/Blueprints/Fish/BP_FishBubble.BP_FishBubble_C" null (`local.Location`) (`local.Rotation`)))
      (bind _asbp_fish_6 (cast `/Game/Blueprints/Fish/BP_Fish_OLD` _returnvalue_6))
      (set `/Game/Blueprints/Fish/BP_Fish_OLD.IsAI` true _asbp_fish_6))
    (:`MantaRay`
      (bind _returnvalue_7 (`AIBlueprintHelperLibrary.SpawnAIFromClass` "/Game/Blueprints/Fish/BP_MantaRay.BP_MantaRay_C" null (`local.Location`) (`local.Rotation`)))
      (bind _asbp_fish_7 (cast `/Game/Blueprints/Fish/BP_Fish_OLD` _returnvalue_7))
      (set `/Game/Blueprints/Fish/BP_Fish_OLD.IsAI` true _asbp_fish_7))))

(fn `Spit`
  (returns (Spitted :type Boolean))
  (locals (LastNonEmptyFishIndex :type Integer) (LastFishType :type Name))
  (bind _returnvalue (`self.K2_GetActorRotation`))
  (bind _fishtype (`self.FishType`))
  (bind _lastfishtype (`local.LastFishType`))
  (bind _returnvalue_2 (`KismetMathLibrary.MakeTransform` (`self.K2_GetActorLocation`) (`self.K2_GetActorRotation`)))
  (bind _returnvalue_3 (+ (`local.LastNonEmptyFishIndex`) 1))
  (bind _returnvalue_4 (+ (`self.K2_GetActorLocation`) (`self.OffsetForSpawnFish`)))
  ;[1 1 1] Get BP_Global (there should only be 1 element in the array of BP_Global.) Get inventory.
  (bind _outactors (`GameplayStatics.GetAllActorsOfClass` "/Game/Blueprints/GameState/BP_Global.BP_Global_C"))
  (for _array_element _outactors
    (bind _inventory (`/Game/Blueprints/GameState/BP_Global.Inventory` _array_element))
    (bind _emptyindex (`self.GetIndexFirstEmptyElement` _inventory))
    (switch `int` _emptyindex
      (:`Default`
        (`KismetSystemLibrary.PrintString` "First empty Index: Default")
        (bind _output_get (set `local.LastNonEmptyFishIndex` (- _emptyindex 2)))
        (set `local.LastFishType` (`|GetArrayItem` _inventory _output_get))
        (`self.SpawnFish` _fishtype _returnvalue_4 _returnvalue)
        (`KismetArrayLibrary.Array_Set` _inventory _returnvalue_3)
        (`self.TransformFish` _lastfishtype _returnvalue_2))
      (:`-1`
        (`KismetSystemLibrary.PrintString` "First Empty Index: -1")
        ;[1 1 1] Inventory is full. Hence, the new player fish index is arr.length - 2
        (bind _output_get_2 (set `local.LastNonEmptyFishIndex` (- (`KismetArrayLibrary.Array_Length` _inventory) 2)))
        (set `local.LastFishType` (`|GetArrayItem` _inventory _output_get_2))
        (`self.SpawnFish` _fishtype _returnvalue_4 _returnvalue)
        (`KismetArrayLibrary.Array_Set` _inventory _returnvalue_3)
        (`self.TransformFish` _lastfishtype _returnvalue_2))
      (:`0`
        (`KismetSystemLibrary.PrintString` "First Empty Index: 0")
        ;[1 1 1] Inventory is empty. No fish to spit out. Return false.
        (return false))
      (:`1`
        ;[1 1 1] The first non-empty index is index 0, which stores the same fish type as the current player's fish type. Hence, spawn current fish type, set fish type at index 0 to None and transform to default fish.
        (`KismetSystemLibrary.PrintString` "First Empty Index: 1")
        (`self.SpawnFish` (`self.FishType`) (+ (`self.K2_GetActorLocation`) (`self.OffsetForSpawnFish`)) (`self.K2_GetActorRotation`))
        (`KismetArrayLibrary.Array_Set` _inventory)
        (`self.TransformFish` "Default" (`KismetMathLibrary.MakeTransform` (`self.K2_GetActorLocation`) (`self.K2_GetActorRotation`)))))
    ;[1 1 1] Update UI for fish inventory
    (bind _foundwidgets (`WidgetBlueprintLibrary.GetAllWidgetsOfClass` "/Game/Blueprints/UI/Gameplay/UI_GamePlay.UI_GamePlay_C"))
    (for _array_element_2 _foundwidgets
      (`/Game/Blueprints/UI/Gameplay/UI_GamePlay.UpdateInventory` _array_element_2)
      (return true))))

(fn `Swallow`
  (params (SmallerFish :type "/Game/Blueprints/Fish/BP_Fish_OLD Object Reference"))
  (returns (Swallowed :type Boolean))
  (bind _fishtype (`/Game/Blueprints/Fish/BP_Fish_OLD.FishType` (`local.SmallerFish`)))
  ;[1 1 1] There should only be one element in the array
  (bind _outactors (`GameplayStatics.GetAllActorsOfClass` "/Game/Blueprints/GameState/BP_Global.BP_Global_C"))
  (for _array_element _outactors
    (bind _inventory (`/Game/Blueprints/GameState/BP_Global.Inventory` _array_element))
    (bind _emptyindex (`self.GetIndexFirstEmptyElement` _inventory))
    (if (!= _emptyindex -1)
      (`KismetArrayLibrary.Array_Set` _inventory _emptyindex _fishtype)
      (`self.TransformFish` _fishtype (`self.GetTransform`))
      (bind _foundwidgets (`WidgetBlueprintLibrary.GetAllWidgetsOfClass` "/Game/Blueprints/UI/Gameplay/UI_GamePlay.UI_GamePlay_C"))
      (for _array_element_2 _foundwidgets
        (`/Game/Blueprints/UI/Gameplay/UI_GamePlay.UpdateInventory` _array_element_2))
      (return true)
      (else
        (return false)))))

(fn `TransformFish`
  (params (FishType :type Name) (Transform :type "Transform Structure"))
  (`KismetSystemLibrary.PrintString` "In TransformFish")
  (`self.K2_DestroyActor`)
  (switch `name` FishType
    (:`Default`
      (bind _returnvalue (`|SpawnActorFromClass` "/Game/Blueprints/Fish/BP_FishDefault.BP_FishDefault_C" (`local.Transform`) "Undefined" "OverrideRootScale" null null))
      (`Controller.Possess` (`GameplayStatics.GetPlayerController` 0) _returnvalue)
      (set `/Game/Blueprints/Fish/BP_Fish_OLD.IsAI` false _returnvalue))
    (:`Glow`
      (bind _returnvalue_2 (`|SpawnActorFromClass` "/Game/Blueprints/Fish/BP_FishGlow.BP_FishGlow_C" (`local.Transform`) "Undefined" "OverrideRootScale" null null))
      (`Controller.Possess` (`GameplayStatics.GetPlayerController` 0) _returnvalue_2)
      (set `/Game/Blueprints/Fish/BP_Fish_OLD.IsAI` false _returnvalue_2))
    (:`Tiny`
      (bind _returnvalue_3 (`|SpawnActorFromClass` "/Game/Blueprints/Fish/BP_FishTiny.BP_FishTiny_C" (`local.Transform`) "Undefined" "OverrideRootScale" null null))
      (`Controller.Possess` (`GameplayStatics.GetPlayerController` 0) _returnvalue_3)
      (set `/Game/Blueprints/Fish/BP_Fish_OLD.IsAI` false _returnvalue_3))
    (:`Starfish`
      (bind _returnvalue_4 (`|SpawnActorFromClass` "/Game/Blueprints/Fish/BP_FishStarfish.BP_FishStarfish_C" (`local.Transform`) "Undefined" "OverrideRootScale" null null))
      (`Controller.Possess` (`GameplayStatics.GetPlayerController` 0) _returnvalue_4)
      (set `/Game/Blueprints/Fish/BP_Fish_OLD.IsAI` false _returnvalue_4))
    (:`Acid`
      (bind _returnvalue_5 (`|SpawnActorFromClass` "/Game/Blueprints/Fish/BP_FishAcid.BP_FishAcid_C" (`local.Transform`) "Undefined" "OverrideRootScale" null null))
      (`Controller.Possess` (`GameplayStatics.GetPlayerController` 0) _returnvalue_5)
      (set `/Game/Blueprints/Fish/BP_Fish_OLD.IsAI` false _returnvalue_5))
    (:`Bubble`
      (bind _returnvalue_6 (`|SpawnActorFromClass` "/Game/Blueprints/Fish/BP_FishBubble.BP_FishBubble_C" (`local.Transform`) "Undefined" "OverrideRootScale" null null))
      (`Controller.Possess` (`GameplayStatics.GetPlayerController` 0) _returnvalue_6)
      (set `/Game/Blueprints/Fish/BP_Fish_OLD.IsAI` false _returnvalue_6))
    (:`MantaRay`
      (bind _returnvalue_7 (`|SpawnActorFromClass` "/Game/Blueprints/Fish/BP_MantaRay.BP_MantaRay_C" (`local.Transform`) "Undefined" "OverrideRootScale" null null))
      (`Controller.Possess` (`GameplayStatics.GetPlayerController` 0) _returnvalue_7)
      (set `/Game/Blueprints/Fish/BP_Fish_OLD.IsAI` false _returnvalue_7))))

(fn `UserConstructionScript`)

(fn `Wander`
  (bind _wandertime (`self.WanderTime`))
  ;[1 1 1] Check for whether wander time should be reset and find new wandering direction (vy and vz)
  (if (or (== _wandertime 0.0) (>= _wandertime (`self.WanderInterval`)))
    ;[1 1 1] Generate random new wander direction
    (bind _output_get (set `self.WanderDirection` (`KismetMathLibrary.Normal` (`KismetMathLibrary.MakeVector` 0.0 (.y (`KismetMathLibrary.RandomUnitVector`)) (.z (`KismetMathLibrary.RandomUnitVector`))))))
    (bind _y (.y _output_get))
    (`KismetSystemLibrary.PrintString` (`KismetStringLibrary.Conv_DoubleToString` _y))
    ;[1 1 1] Set facing direction
    (bind _output_get_2 (set `self.FacingRight` (> _y 0.0)))
    (`KismetSystemLibrary.PrintString` (`KismetStringLibrary.Conv_BoolToString` _output_get_2))
    ;[1 1 1] Reset wander time
    (set `self.WanderTime` 0.0))
  ;[1 1 1] Update WanderTime
  (set `self.WanderTime` (+ (`self.WanderTime`) (`GameplayStatics.GetWorldDeltaSeconds`)))
  ;[1 1 1] Update location
  (`self.K2_SetActorLocation` (+ (`self.K2_GetActorLocation`) (* (`self.WanderDirection`) (`self.Speed`)))))