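; Test enemy actor that chases the first player character when it comes within range.
; Each Tick it measures the distance to the player and, inside a fixed radius, steps along the normalized direction by Speed.
; Movement sets location directly without sweeping, so it ignores collision and is not scaled by delta time.
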(event `self.ReceiveActorBeginOverlap`
  (params (OtherActor :type "Actor Object Reference")))

(event `self.ReceiveTick`
  (params (DeltaSeconds :type "Float (single-precision)"))
  (bind _returnvalue (- (`self.K2_GetActorLocation` (`GameplayStatics.GetPlayerCharacter` 0)) (`self.K2_GetActorLocation`)))
  (if (< (`KismetMathLibrary.VSize` _returnvalue) 500.0)
    (`self.K2_SetActorLocation` (+ (`self.K2_GetActorLocation`) (* (`KismetMathLibrary.Normal` _returnvalue) (`self.Speed`))))))

(fn `UserConstructionScript`)