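; Manta ray fish Blueprint that moves on input and can dive into sand.
; BeginPlay sets its type, speed and scale, the construction script flags it as AI, and axis inputs move it in Y and Z with swept location offsets.
; Pressing Ability switches BP_Sand meshes overlapping its trigger capsule to query-only collision.
; Releasing it restores query-and-physics collision on every BP_Sand in the level.
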(event `self.ReceiveBeginPlay`
  (`parent.ReceiveBeginPlay`)
  (set `self.FishType` "MantaRay")
  (set `self.Speed` 1.0)
  (bind _output_get (set `self.Size` 0.5))
  (`self.SetActorScale3D` (`KismetMathLibrary.MakeVector` _output_get _output_get _output_get)))

(event `InputAction|Ability`
  (params (Key :type "Key Structure"))
  (:`Pressed`
    (`self.Dive`))
  (:`Released`
    (bind _outactors (`GameplayStatics.GetAllActorsOfClass` "/Game/Blueprints/Objects/BP_Sand.BP_Sand_C"))
    (for _array_element _outactors
      (`PrimitiveComponent.SetCollisionEnabled` (`/Game/Blueprints/Objects/BP_Sand.TriggerMesh` _array_element) "QueryAndPhysics"))))

(event `InputAxis|MoveHorizontal`
  (params (AxisValue :type "Float (single-precision)"))
  (`self.K2_SetActorLocation` (+ (`self.K2_GetActorLocation`) (* (`KismetMathLibrary.MakeVector` 0.0 AxisValue) 3.0)) true))

(event `InputAxis|MoveVertical`
  (params (AxisValue :type "Float (single-precision)"))
  (`self.K2_SetActorLocation` (+ (`self.K2_GetActorLocation`) (* (`KismetMathLibrary.MakeVector` 0.0 0.0 AxisValue) 3.0)) true))

(fn `Dive`
  (bind _triggercapsule (`self.TriggerCapsule`))
  (bind _outactors (`KismetSystemLibrary.CapsuleOverlapActors` (`SceneComponent.K2_GetComponentLocation` _triggercapsule) (`CapsuleComponent.CapsuleRadius` _triggercapsule) (`CapsuleComponent.GetScaledCapsuleHalfHeight` _triggercapsule) (`|MakeArray` "ObjectTypeQuery9" :!type "EObjectTypeQuery Enum")))
  (for _array_element _outactors
    (bind _asbp_sand (cast `/Game/Blueprints/Objects/BP_Sand` _array_element))
    (`PrimitiveComponent.SetCollisionEnabled` (`/Game/Blueprints/Objects/BP_Sand.TriggerMesh` _asbp_sand) "QueryOnly")))

(fn `UserConstructionScript`
  (set `self.IsAI` true))