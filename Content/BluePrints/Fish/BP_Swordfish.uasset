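; Swordfish Blueprint for a fish that sets its type, speed and scale at BeginPlay and has a seaweed-cutting ability.
; The Ability input calls CutSeaweed, which runs a capsule overlap at TriggerCapsule filtered to one object type and destroys the actors found.
; After a successful cut, it casts itself to BP_Fish to set DeltaV and vertical and lateral velocity limits, with debug drawing and prints left in.
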(event `self.ReceiveBeginPlay`
  (`parent.ReceiveBeginPlay`)
  (set `self.FishType` "Swordfish")
  (set `self.Speed` 3.25)
  (bind _output_get (set `self.Size` 0.99))
  (`self.SetActorScale3D` (`KismetMathLibrary.MakeVector` _output_get _output_get _output_get)))

(event `InputAction|Ability`
  (params (Key :type "Key Structure"))
  (:`Pressed`
    (`self.CutSeaweed`)))

(fn `CutSeaweed`
  (bind _triggercapsule (`self.TriggerCapsule`))
  (bind _returnvalue (`SceneComponent.K2_GetComponentLocation` _triggercapsule))
  (bind _returnvalue_2 (`CapsuleComponent.GetScaledCapsuleHalfHeight` _triggercapsule))
  (bind _capsuleradius (`CapsuleComponent.CapsuleRadius` _triggercapsule))
  (`KismetSystemLibrary.DrawDebugCapsule` _returnvalue _returnvalue_2 _capsuleradius (struct) (struct :`R` 0.670283 :`G` 1.0 :`B` 0.646556 :`A` 1.0))
  (bind (_outactors _returnvalue_3) (`KismetSystemLibrary.CapsuleOverlapActors` _returnvalue _capsuleradius _returnvalue_2 (`|MakeArray` "ObjectTypeQuery13" :!type "EObjectTypeQuery Enum")))
  (if _returnvalue_3
    (for _array_element _outactors
      (`self.K2_DestroyActor` _array_element))
    (bind _asbp_fish (cast `/Game/BluePrints/Fish/BP_Fish` self)
      (:`then`
        (set `/Game/BluePrints/Fish/BP_Fish.delta_v` 0.4 _asbp_fish)
        (set `/Game/BluePrints/Fish/BP_Fish.VyMax` 5.0 _asbp_fish)
        (set `/Game/BluePrints/Fish/BP_Fish.VzMax` 5.0 _asbp_fish)
        (`KismetSystemLibrary.PrintString` "...readjusting"))
      (:`CastFailed`
        (`KismetSystemLibrary.PrintString` "HUH??")))))

(fn `UserConstructionScript`
  (`parent.UserConstructionScript`))