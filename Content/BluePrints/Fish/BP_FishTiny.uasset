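; BP_FishTiny is the tiny fish variant, a child Blueprint that configures variables for its fish type.
; On BeginPlay it calls the parent, then sets the fish type to Tiny, assigns a speed and copies that speed into size.
; Size becomes the actor's uniform 3D scale, so scale follows the speed value.
; It adds no overlap, tick or construction logic of its own.
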(event `self.ReceiveBeginPlay`
  (`parent.ReceiveBeginPlay`)
  (set `self.FishType` "Tiny")
  (bind _output_get (set `self.Speed` 0.25))
  (bind _output_get_2 (set `self.Size` _output_get))
  (`self.SetActorScale3D` (`KismetMathLibrary.MakeVector` _output_get_2 _output_get_2 _output_get_2)))

(fn `UserConstructionScript`
  (`parent.UserConstructionScript`))