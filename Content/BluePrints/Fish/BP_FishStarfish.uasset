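; Player-controlled starfish fish type, built on a parent fish class, that can break off up to two legs and reabsorb them.
; Physics velocity drives grounded jumps, while swept offsets move the body and every spawned BP_StarfishLeg sideways together along Y.
; The ability spawns legs beside the body.
; Tick uses trigger-capsule overlaps to destroy touched legs, decrement the active count, and refresh OnGround from WorldStatic contact.
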(event `self.ReceiveBeginPlay`
  (`parent.ReceiveBeginPlay`)
  (set `self.FishType` "Starfish")
  (set `self.Speed` 1.0))

(event `InputAxis|MoveVertical`
  (params (AxisValue :type "Float (single-precision)"))
  (bind _capsulecomponent (`self.CapsuleComponent`))
  ;[1 1 1] Movement
  (if (and (> AxisValue 0.0) (`self.onGround`))
    (`PrimitiveComponent.SetPhysicsAngularVelocityInDegrees` _capsulecomponent (0.0 0.0 0.0) false "None")
    (`PrimitiveComponent.SetPhysicsLinearVelocity` _capsulecomponent (`KismetMathLibrary.MakeVector` 0.0 0.0 130.0) true "None")
    (set `self.onGround` false)))

(event `InputAxis|MoveHorizontal`
  (params (AxisValue :type "Float (single-precision)"))
  ;[1 1 1] Movement
  (`self.K2_SetActorLocation` (+ (`self.K2_GetActorLocation`) (`KismetMathLibrary.MakeVector` 0.0 (* AxisValue 2.0))) true)
  (bind _outactors (`GameplayStatics.GetAllActorsOfClass` "/Game/BluePrints/Fish/BP_StarfishLeg.BP_StarfishLeg_C"))
  (for _array_element _outactors
    (`PrimitiveComponent.SetPhysicsAngularVelocityInDegrees` (`/Game/BluePrints/Fish/BP_StarfishLeg.LegCollider` _array_element) (0.0 0.0 0.0) false "None")
    (`self.K2_SetActorLocation` _array_element (+ (`self.K2_GetActorLocation` _array_element) (`KismetMathLibrary.MakeVector` 0.0 (* AxisValue 2.0))) true false)))

(event `InputAction|Ability`
  (params (Key :type "Key Structure"))
  ;[1 1 1] Ability: Break off legs
  (:`Pressed`
    (if (< (`self.activeLegs`) 2)
      (`|SpawnActorFromClass` "/Game/BluePrints/Fish/BP_StarfishLeg.BP_StarfishLeg_C" (`KismetMathLibrary.MakeTransform` (+ (`self.K2_GetActorLocation`) (`KismetMathLibrary.MakeVector` 0.0 2.0 1.0))) "AdjustIfPossibleButAlwaysSpawn" "OverrideRootScale" null null)
      (set `self.activeLegs` (+ (`self.activeLegs`) 1)))))

(event `self.ReceiveTick`
  (params (DeltaSeconds :type "Float (single-precision)"))
  (bind _triggercapsule (`self.TriggerCapsule`))
  (bind _returnvalue (`SceneComponent.K2_GetComponentLocation` _triggercapsule))
  (bind _returnvalue_2 (`CapsuleComponent.GetScaledCapsuleHalfHeight` _triggercapsule))
  (bind _capsuleradius (`CapsuleComponent.CapsuleRadius` _triggercapsule))
  ;[1 1 1] Leg Collision (absorb leg)
  (`parent.ReceiveTick` DeltaSeconds)
  (bind (_outactors _returnvalue_3) (`KismetSystemLibrary.CapsuleOverlapActors` _returnvalue _capsuleradius _returnvalue_2 (`|MakeArray` "ObjectTypeQuery9" :!type "EObjectTypeQuery Enum") "/Game/BluePrints/Fish/BP_StarfishLeg.BP_StarfishLeg_C" (`|MakeArray` (`GameplayStatics.GetPlayerCharacter` 0) :!type "Actor Object Reference")))
  (if _returnvalue_3
    (for _array_element _outactors
      (`self.K2_DestroyActor` _array_element)
      (set `self.activeLegs` (- (`self.activeLegs`) 1))
      (bind (_outactors_2 _returnvalue_4) (`KismetSystemLibrary.CapsuleOverlapActors` _returnvalue _capsuleradius _returnvalue_2 (`|MakeArray` "ObjectTypeQuery1" :!type "EObjectTypeQuery Enum") null (`|MakeArray` (`GameplayStatics.GetPlayerCharacter` 0) :!type "Actor Object Reference") :!label _label))
      (set `self.onGround` _returnvalue_4))
    (else
      (goto _label))))

(fn `UserConstructionScript`
  (`parent.UserConstructionScript`))