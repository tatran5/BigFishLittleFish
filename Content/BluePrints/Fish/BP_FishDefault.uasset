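; BP_FishDefault is a fish Blueprint variant that sets up the default, non-AI fish, likely one a player controls.
; On BeginPlay it runs the parent logic, then sets its type to Default, turns off the AI flag and assigns a size.
; That size uniformly scales the mesh in world space; all other behavior comes from the parent class.
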(event `self.ReceiveBeginPlay`
  (`parent.ReceiveBeginPlay`)
  (set `self.FishType` "Default")
  (set `self.IsAI` false)
  (bind _output_get (set `self.Size` 2.0))
  (`SceneComponent.SetWorldScale3D` (`self.Mesh`) (`KismetMathLibrary.MakeVector` _output_get _output_get _output_get)))

(fn `UserConstructionScript`
  (`parent.UserConstructionScript`))