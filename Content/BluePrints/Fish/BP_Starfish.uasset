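; BP_Starfish is a player-controlled starfish that moves in the Y-Z plane and can spawn detachable-style BP_StarfishLeg actors.
; Vertical input only lifts it while OnGround is set, zeroing collider spin first; nothing here clears that flag.
; Horizontal input sweeps the body sideways and shifts every leg actor in the world alike, stopping their spin.
; The Ability input spawns a leg beside the starfish, capped at two.
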(event `InputAxis|MoveVertical`
  (params (AxisValue :type "Float (single-precision)"))
  (if (and (> AxisValue 0.0) (`self.onGround`))
    (`PrimitiveComponent.SetPhysicsAngularVelocityInDegrees` (`self.StarfishCollider`) (0.0 0.0 0.0) false "None")
    (`self.K2_SetActorLocation` (+ (`self.K2_GetActorLocation`) (`KismetMathLibrary.MakeVector` 0.0 0.0 (* AxisValue 5.0))) true)
    (set `self.onGround` true)))

(event `InputAxis|MoveHorizontal`
  (params (AxisValue :type "Float (single-precision)"))
  (`self.K2_SetActorLocation` (+ (`self.K2_GetActorLocation`) (`KismetMathLibrary.MakeVector` 0.0 (* AxisValue 2.0))) true)
  (bind _outactors (`GameplayStatics.GetAllActorsOfClass` "/Game/BluePrints/Fish/BP_StarfishLeg.BP_StarfishLeg_C"))
  (for _array_element _outactors
    (`PrimitiveComponent.SetPhysicsAngularVelocityInDegrees` (`/Game/BluePrints/Fish/BP_StarfishLeg.LegCollider` _array_element) (0.0 0.0 0.0) false "None")
    (`self.K2_SetActorLocation` _array_element (+ (`self.K2_GetActorLocation` _array_element) (`KismetMathLibrary.MakeVector` 0.0 (* AxisValue 2.0))) true false)))

(event `InputAction|Ability`
  (params (Key :type "Key Structure"))
  (:`Pressed`
    (if (< (`self.activeLegs`) 2)
      (`|SpawnActorFromClass` "/Game/BluePrints/Fish/BP_StarfishLeg.BP_StarfishLeg_C" (`KismetMathLibrary.MakeTransform` (+ (`self.K2_GetActorLocation`) (`KismetMathLibrary.MakeVector` 0.0 2.0 1.0))) "AdjustIfPossibleButAlwaysSpawn" "OverrideRootScale" null null)
      (set `self.activeLegs` (+ (`self.activeLegs`) 1)))))

(fn `UserConstructionScript`
  (set `self.onGround` true)
  (set `self.activeLegs` 0))