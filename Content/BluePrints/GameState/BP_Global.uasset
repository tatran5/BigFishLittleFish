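; BP_Global is a game-state Blueprint that tracks the player's remaining lives.
; DecreaseLives subtracts one from LivesLeft while it is above zero, then has every top-level UI_GamePlay widget refresh its lives display.
; A call made with no lives left opens the GameOver_Lose level instead.
; The event graph and construction script are empty.
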(fn `DecreaseLives`
  (`KismetSystemLibrary.PrintString` "In DecraseLives")
  (if (> (`self.LivesLeft`) 0)
    (set `self.LivesLeft` (- (`self.LivesLeft`) 1))
    (bind _foundwidgets (`WidgetBlueprintLibrary.GetAllWidgetsOfClass` "/Game/BluePrints/UI/Gameplay/UI_GamePlay.UI_GamePlay_C"))
    (for _array_element _foundwidgets
      (`/Game/BluePrints/UI/Gameplay/UI_GamePlay.UpdateLivesWidget` _array_element))
    (else
      (`GameplayStatics.OpenLevel` "GameOver_Lose"))))

(fn `UserConstructionScript`)