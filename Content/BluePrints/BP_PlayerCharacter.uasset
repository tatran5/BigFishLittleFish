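; Player character for a 2D-plane game that collects fish and avoids enemies.
; Axis inputs move it with swept location offsets in Y and Z, with horizontal input also setting a FacingRight flag.
; Each tick it draws a debug capsule and queries TriggerCapsule overlaps, destroying any fish found.
; Only when no fish overlap does it check for enemies, which teleport it to a fixed position.
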(event `InputAxis|MoveVertical`
  (params (AxisValue :type "Float (single-precision)"))
  ;[1 1 1] Movement
  (`self.K2_SetActorLocation` (+ (`self.K2_GetActorLocation`) (`KismetMathLibrary.MakeVector` 0.0 0.0 (* AxisValue 3.0))) true))

(event `InputAxis|MoveHorizontal`
  (params (AxisValue :type "Float (single-precision)"))
  ;[1 1 1] Movement
  (set `self.facingRight` (> AxisValue 0.0))
  (`self.K2_SetActorLocation` (+ (`self.K2_GetActorLocation`) (`KismetMathLibrary.MakeVector` 0.0 (* AxisValue 3.0))) true))

(event `self.ReceiveTick`
  (params (DeltaSeconds :type "Float (single-precision)"))
  (bind _triggercapsule (`self.TriggerCapsule`))
  (bind _triggercapsule_2 (`self.TriggerCapsule`))
  (bind _returnvalue (`SceneComponent.K2_GetComponentLocation` _triggercapsule))
  (bind _returnvalue_2 (`CapsuleComponent.GetScaledCapsuleHalfHeight` _triggercapsule))
  (bind _capsuleradius (`CapsuleComponent.CapsuleRadius` _triggercapsule))
  ;[1 1 1] CollisionDetectionFish
  (`KismetSystemLibrary.DrawDebugCapsule` _returnvalue _returnvalue_2 _capsuleradius (struct) (struct :`R` 0.670283 :`G` 1.0 :`B` 0.646556 :`A` 1.0))
  (bind (_outactors _returnvalue_3) (`KismetSystemLibrary.CapsuleOverlapActors` _returnvalue _capsuleradius _returnvalue_2 (`|MakeArray` "ObjectTypeQuery8" :!type "EObjectTypeQuery Enum") null (`|MakeArray` (`GameplayStatics.GetPlayerCharacter` 0) :!type "Actor Object Reference")))
  (if _returnvalue_3
    (for _array_element _outactors
      (`self.K2_DestroyActor` _array_element))
    (else
      ;[1 1 1] CollisionDetectionEnemy
      (bind (_outactors_2 _returnvalue_4) (`KismetSystemLibrary.CapsuleOverlapActors` (`SceneComponent.K2_GetComponentLocation` _triggercapsule_2) (`CapsuleComponent.CapsuleRadius` _triggercapsule_2) (`CapsuleComponent.GetScaledCapsuleHalfHeight` _triggercapsule_2) (`|MakeArray` "ObjectTypeQuery7" :!type "EObjectTypeQuery Enum") null (`|MakeArray` (`GameplayStatics.GetPlayerCharacter` 0) :!type "Actor Object Reference")))
      (if _returnvalue_4
        (`self.K2_SetActorLocation` (-170.0 0.0 112.0) false true)))))

(fn `UserConstructionScript`
  (set `self.facingRight` true))