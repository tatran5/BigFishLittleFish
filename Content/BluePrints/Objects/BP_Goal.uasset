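; BP_Goal is the level goal: any hit on its GoalCollider records the level result and opens GameOver_Win.
; It loads the existing "Data" BP_Data save and writes BP_Global's bonus stars plus one into LevelResults, indexed by the numeric level name.
; The win screen opens only after a successful save, with debug prints for results and failures.
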(event `self.GoalCollider.OnComponentHit`
  (params (HitComponent :type "PrimitiveComponent Object Reference") (OtherActor :type "Actor Object Reference") (OtherComp :type "PrimitiveComponent Object Reference") (NormalImpulse :type "Vector Structure") (Hit :type "HitResult Structure (by ref)"))
  (bind _returnvalue (`GameplayStatics.GetCurrentLevelName` true))
  (bind _outactors (`GameplayStatics.GetAllActorsOfClass` "/Game/Blueprints/GameState/BP_Global.BP_Global_C"))
  (bind _returnvalue_2 (`GameplayStatics.DoesSaveGameExist` "Data"))
  (if _returnvalue_2
    ;[1 1 1] Update the last level cleared and the number of stars acquired for this level
    (bind _returnvalue_3 (`GameplayStatics.LoadGameFromSlot` "Data"))
    (bind _asbp_data (cast `/Game/Blueprints/GameState/BP_Data` _returnvalue_3)
      (:`then`
        (bind _levelresults (`/Game/Blueprints/GameState/BP_Data.LevelResults` _asbp_data))
        (`KismetArrayLibrary.Array_Set` _levelresults (- (`KismetStringLibrary.Conv_StringToInt` _returnvalue) 1) (+ (`/Game/Blueprints/GameState/BP_Global.BonusStarsAcquired` (`|GetArrayItem` _outactors)) 1))
        (bind _returnvalue_4 (`GameplayStatics.SaveGameToSlot` _asbp_data "Data"))
        (if _returnvalue_4
          (`KismetSystemLibrary.PrintString` "Saved")
          (for _array_element _levelresults
            (`KismetSystemLibrary.PrintString` (`KismetStringLibrary.Conv_IntToString` _array_element) true true (struct :`R` 1.0 :`G` 0.857059 :`A` 1.0) 10.0))
          (`GameplayStatics.OpenLevel` "GameOver_Win")
          (else
            (`KismetSystemLibrary.PrintString` "Can't save"))))
      (:`CastFailed`
        (`KismetSystemLibrary.PrintString` "Can't cast data to BP_Data")))
    (else
      (`KismetSystemLibrary.PrintString` "Cannot find data. Cannot Save"))))

(fn `UserConstructionScript`)