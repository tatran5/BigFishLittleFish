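; BP_Spikes is a hazard that pops BP_Box bubbles and costs the player's fish a life on contact.
; Each Tick it runs two box overlap queries sized to PlatformBoxCollider, which construction sets to WorldStatic, instead of using overlap events.
; Non-AI BP_Fish hits decrement lives on BP_Global and play the lose-life animation, with no cooldown in this graph.
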(event `self.ReceiveTick`
  (params (DeltaSeconds :type "Float (single-precision)"))
  (bind _platformboxcollider (`self.PlatformBoxCollider`))
  (bind _returnvalue (`BoxComponent.GetScaledBoxExtent` _platformboxcollider))
  (bind _returnvalue_2 (`SceneComponent.K2_GetComponentLocation` _platformboxcollider))
  ;[1 1 1] Pop Bubble
  (`parent.ReceiveTick` DeltaSeconds)
  (bind _outactors (`KismetSystemLibrary.BoxOverlapActors` _returnvalue_2 _returnvalue (`|MakeArray` "ObjectTypeQuery2" :!type "EObjectTypeQuery Enum") "/Game/BluePrints/Objects/BP_Box.BP_Box_C"))
  (for _array_element _outactors
    (bind _asbp_box (cast `/Game/BluePrints/Objects/BP_Box` _array_element))
    (`/Game/BluePrints/Objects/BP_Box.Pop` _asbp_box))
  (bind _outactors_2 (`KismetSystemLibrary.BoxOverlapActors` _returnvalue_2 _returnvalue (`|MakeArray` "ObjectTypeQuery8" :!type "EObjectTypeQuery Enum") "/Game/BluePrints/Fish/BP_Fish.BP_Fish_C"))
  (for _array_element_2 _outactors_2
    (bind _asbp_fish (cast `/Game/BluePrints/Fish/BP_Fish` _array_element_2))
    (if (not (`/Game/BluePrints/Fish/BP_Fish.IsAI` _asbp_fish))
      (bind _returnvalue_3 (`GameplayStatics.GetActorOfClass` "/Game/BluePrints/GameState/BP_Global.BP_Global_C"))
      (`/Game/BluePrints/GameState/BP_Global.DecreaseLives` _returnvalue_3)
      (`/Game/BluePrints/Fish/BP_Fish.AnimateLoseLife` _asbp_fish))))

(fn `UserConstructionScript`
  (`parent.UserConstructionScript`)
  (`PrimitiveComponent.SetCollisionObjectType` (`self.PlatformBoxCollider`) "ECC_WorldStatic"))