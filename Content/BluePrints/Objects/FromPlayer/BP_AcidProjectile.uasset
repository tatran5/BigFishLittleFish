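; BP_AcidProjectile is an acid projectile that dissolves wood by destroying BP_Wood actors it touches.
; Each tick, after the parent tick, it runs a sphere overlap at its ProjectileCollider against WorldStatic objects, ignoring the player character.
; On any hit it destroys at most one overlapped BP_Wood, then destroys itself.
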(event `self.ReceiveTick`
  (params (DeltaSeconds :type "Float (single-precision)"))
  (bind _projectilecollider (`self.ProjectileCollider`))
  (`parent.ReceiveTick` DeltaSeconds)
  (bind (_outactors _returnvalue) (`KismetSystemLibrary.SphereOverlapActors` (`SceneComponent.K2_GetComponentLocation` _projectilecollider) (`SphereComponent.SphereRadius` _projectilecollider) (`|MakeArray` "ObjectTypeQuery1" :!type "EObjectTypeQuery Enum") null (`|MakeArray` (`GameplayStatics.GetPlayerCharacter` 0) :!type "Actor Object Reference")))
  (if _returnvalue
    (for _array_element _outactors
      (cast `/Game/BluePrints/Objects/BP_Wood` _array_element)
      (`self.K2_DestroyActor` _array_element)
      (break))
    (`self.K2_DestroyActor`)))

(fn `UserConstructionScript`
  (`parent.UserConstructionScript`))