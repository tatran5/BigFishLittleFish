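; BP_Bubble is a projectile actor that applies a bubble effect to a BP_Box it touches.
; Each Tick it runs sphere overlaps at its ProjectileCollider's position and radius, ignoring the player character, instead of using overlap events.
; A WorldDynamic box hit calls Bubble on the first box found and destroys the projectile.
; Otherwise, any WorldStatic overlap simply destroys it.
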(event `self.ReceiveTick`
  (params (DeltaSeconds :type "Float (single-precision)"))
  (bind _projectilecollider (`self.ProjectileCollider`))
  (bind _returnvalue (`SceneComponent.K2_GetComponentLocation` _projectilecollider))
  (bind _array (`|MakeArray` (`GameplayStatics.GetPlayerCharacter` 0) :!type "Actor Object Reference"))
  (bind _sphereradius (`SphereComponent.SphereRadius` _projectilecollider))
  (`parent.ReceiveTick` 0.0)
  (bind (_outactors _returnvalue_2) (`KismetSystemLibrary.SphereOverlapActors` _returnvalue _sphereradius (`|MakeArray` "ObjectTypeQuery2" :!type "EObjectTypeQuery Enum") "/Game/Blueprints/Objects/BP_Box.BP_Box_C" _array))
  (if _returnvalue_2
    (for _array_element _outactors
      (bind _asbp_box (cast `/Game/Blueprints/Objects/BP_Box` _array_element))
      (`/Game/Blueprints/Objects/BP_Box.Bubble` _asbp_box)
      (break))
    (`self.K2_DestroyActor` :!label _label)
    (else
      (bind (_outactors_2 _returnvalue_3) (`KismetSystemLibrary.SphereOverlapActors` _returnvalue _sphereradius (`|MakeArray` "ObjectTypeQuery1" :!type "EObjectTypeQuery Enum") null _array))
      (if _returnvalue_3
        (goto _label)))))

(fn `UserConstructionScript`
  (`parent.UserConstructionScript`))