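; BP_Box is a box that can be encased in a bubble, making it float upward until a fish pops it.
; Bubble disables gravity, shows the sphere and enables the overlap trigger; Pop reverses this when any BP_Fish overlaps it.
; While bubbled, Tick sweeps it up by a fixed per-frame step, unscaled by delta time.
; Tick also shows PlatformBoxCollider only if the player's fish type is Bubble or Acid.
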(event `self.ReceiveTick`
  (params (DeltaSeconds :type "Float (single-precision)"))
  (`parent.ReceiveTick` DeltaSeconds)
  (if (`self.bubbled`)
    (`self.K2_SetActorLocation` (+ (`self.K2_GetActorLocation`) (0.0 0.0 2.0)) true)
    (bind _asbp_fish (cast `/Game/BluePrints/Fish/BP_Fish` (`GameplayStatics.GetPlayerCharacter` 0)))
    (bind _fishtype (`/Game/BluePrints/Fish/BP_Fish.FishType` _asbp_fish))
    (if (or (== _fishtype "Bubble") (== _fishtype "Acid"))
      (`SceneComponent.SetHiddenInGame` (`self.PlatformBoxCollider`) false false)
      (else
        (`SceneComponent.SetHiddenInGame` (`self.PlatformBoxCollider`) true false)))))

(event `self.BubbleCollider.OnComponentBeginOverlap`
  (params (OverlappedComponent :type "PrimitiveComponent Object Reference") (OtherActor :type "Actor Object Reference") (OtherComp :type "PrimitiveComponent Object Reference") (OtherBodyIndex :type Integer) (bFromSweep :type Boolean) (SweepResult :type "HitResult Structure (by ref)"))
  (cast `/Game/BluePrints/Fish/BP_Fish` OtherActor)
  (`self.Pop`))

(fn `Bubble`
  (`PrimitiveComponent.SetEnableGravity` (`self.PlatformBoxCollider`) false)
  (set `self.bubbled` true)
  (`PrimitiveComponent.SetCollisionEnabled` (`self.BubbleCollider`) "QueryOnly")
  (`SceneComponent.SetVisibility` (`self.SphereMesh`) true false))

(fn `Pop`
  (bind _spheremesh (`self.SphereMesh`))
  (`PrimitiveComponent.SetEnableGravity` (`self.PlatformBoxCollider`) true)
  (set `self.bubbled` false)
  (`PrimitiveComponent.SetCollisionEnabled` (`self.BubbleCollider`) "NoCollision")
  (`PrimitiveComponent.SetCollisionEnabled` _spheremesh "NoCollision")
  (`SceneComponent.SetVisibility` _spheremesh false false))

(fn `UserConstructionScript`
  (`parent.UserConstructionScript`)
  (set `self.bubbled` false)
  (`PrimitiveComponent.SetCollisionEnabled` (`self.BubbleCollider`) "NoCollision")
  (`PrimitiveComponent.SetCollisionEnabled` (`self.SphereMesh`) "NoCollision"))