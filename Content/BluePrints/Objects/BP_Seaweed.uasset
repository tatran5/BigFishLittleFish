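; BP_Seaweed is a seaweed obstacle that slows the player's fish while its box detects an overlap.
; Each Tick runs a box overlap query on one object type and writes reduced or normal acceleration and speed limits to the player's BP_Fish.
; The normal values are written whenever the box is empty, so every instance overwrites them each frame.
; Tick also shows TriggerMesh only when the player's FishType is SwordFish.
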(event `self.ReceiveBeginPlay`
  (set `self.NextExecution` 20.0))

(event `self.ReceiveTick`
  (params (DeltaSeconds :type "Float (single-precision)"))
  (`self.CheckForPlayer`)
  (bind _asbp_fish (cast `/Game/Blueprints/Fish/BP_Fish` (`GameplayStatics.GetPlayerCharacter` 0))
    (:`then`
      (if (== (`/Game/Blueprints/Fish/BP_Fish.FishType` _asbp_fish) "SwordFish")
        (`SceneComponent.SetHiddenInGame` (`self.TriggerMesh`) false true)
        (else
          (`SceneComponent.SetHiddenInGame` (`self.TriggerMesh`) true true))))
    (:`CastFailed`
      (`KismetSystemLibrary.PrintString` "Cast failed!"))))

(fn `CheckForPlayer`
  (bind _returnvalue (`GameplayStatics.GetPlayerCharacter` 0))
  (bind _box (`self.Box`))
  (bind (_outactors _returnvalue_2) (`KismetSystemLibrary.BoxOverlapActors` (`SceneComponent.K2_GetComponentLocation` _box) (`BoxComponent.GetScaledBoxExtent` _box) (`|MakeArray` "ObjectTypeQuery8" :!type "EObjectTypeQuery Enum")))
  (if _returnvalue_2
    (bind _asbp_fish (cast `/Game/Blueprints/Fish/BP_Fish` _returnvalue))
    (set `/Game/Blueprints/Fish/BP_Fish.delta_v` 0.22 _asbp_fish)
    (set `/Game/Blueprints/Fish/BP_Fish.VyMax` 1.0 _asbp_fish)
    (set `/Game/Blueprints/Fish/BP_Fish.VzMax` 1.0 _asbp_fish)
    (else
      (bind _asbp_fish_2 (cast `/Game/Blueprints/Fish/BP_Fish` _returnvalue))
      (set `/Game/Blueprints/Fish/BP_Fish.delta_v` 0.4 _asbp_fish_2)
      (set `/Game/Blueprints/Fish/BP_Fish.VyMax` 5.0 _asbp_fish_2)
      (set `/Game/Blueprints/Fish/BP_Fish.VzMax` 5.0 _asbp_fish_2))))

(fn `UserConstructionScript`)