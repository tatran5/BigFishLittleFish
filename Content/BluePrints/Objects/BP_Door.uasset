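; BP_Door is a sliding door that opens while any of its connected buttons is pressed and closes otherwise.
; Each Tick it ORs the buttons' Pressed states, then steps the actor by Speed with a sweep, independent of DeltaSeconds.
; Direction selects vertical (Z) or horizontal (Y) travel, clamped between the position saved in the construction script and that position plus Range.
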(event `self.ReceiveTick`
  (params (DeltaSeconds :type "Float (single-precision)"))
  (bind _direction (`self.direction`))
  (bind _speed (`self.speed`))
  (bind _y (.y (`self.K2_GetActorLocation`)))
  (bind _z (.z (`self.K2_GetActorLocation`)))
  (bind _x (.x (`self.initialPos`)))
  (bind _y_2 (.y (`self.initialPos`)))
  (bind _z_2 (.z (`self.initialPos`)))
  (bind _returnvalue (+ (`self.range`) _y_2))
  (bind _returnvalue_2 (+ (`self.range`) _z_2))
  ;[1 1 1] Open and Close Behavior
  (`parent.ReceiveTick` DeltaSeconds)
  ;;[1 1 1] First iterate through all buttons to see if one is pressed
  (for (_array_element _array_index) (`self.connectedButtons`)
    (if (== _array_index 0)
      (bind _pressed (`/Game/Blueprints/Objects/BP_Button.pressed` _array_element))
      (set `self.opening` (or false _pressed))
      (else
        (set `self.opening` (or (`self.opening`) _pressed)))))
  (if (`self.opening`)
    (switch `int` _direction
      (:`Default`
        (`self.K2_SetActorLocation` (`KismetMathLibrary.MakeVector` _x _y_2 (`KismetMathLibrary.FClamp` (+ _z _speed) _z_2 _returnvalue_2)) true :!label _label))
      (:`0`
        (goto _label))
      (:`1`
        (`self.K2_SetActorLocation` (`KismetMathLibrary.MakeVector` _x (`KismetMathLibrary.FClamp` (+ _y _speed) _y_2 _returnvalue) _z_2) true :!label _label_2))
      (:`2`
        (goto _label_2)))
    (else
      (switch `int` _direction
        (:`Default`
          (`self.K2_SetActorLocation` (`KismetMathLibrary.MakeVector` _x _y_2 (`KismetMathLibrary.FClamp` (- _z _speed) _z_2 _returnvalue_2)) true :!label _label_3))
        (:`0`
          (goto _label_3))
        (:`1`
          (`self.K2_SetActorLocation` (`KismetMathLibrary.MakeVector` _x (`KismetMathLibrary.FClamp` (- _y _speed) _y_2 _returnvalue) _z_2) true))))))

(fn `UserConstructionScript`
  (`parent.UserConstructionScript`)
  (set `self.initialPos` (`self.K2_GetActorLocation`)))