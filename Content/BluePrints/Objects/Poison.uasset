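; Poison hazard object that periodically checks for a player inside its Box volume, with only a debug response so far.
; Tick decrements a frame counter and runs CheckForPlayer about every 40 frames, so the interval depends on frame rate.
; CheckForPlayer runs a box overlap query matching the Box bounds against one object type and prints "OUCH" on a hit, applying no damage.
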(event `self.ReceiveBeginPlay`
  (set `self.NextExecution` 40.0))

(event `self.ReceiveTick`
  (params (DeltaSeconds :type "Float (single-precision)"))
  (if (>= (`self.NextExecution`) 1.0)
    (set `self.NextExecution` (- (`self.NextExecution`) 1.0))
    (else
      (`self.CheckForPlayer`)
      (set `self.NextExecution` 40.0))))

(fn `CheckForPlayer`
  (bind _box (`self.Box`))
  (bind (_outactors _returnvalue) (`KismetSystemLibrary.BoxOverlapActors` (`SceneComponent.K2_GetComponentLocation` _box) (`BoxComponent.GetScaledBoxExtent` _box) (`|MakeArray` "ObjectTypeQuery8" :!type "EObjectTypeQuery Enum")))
  (if _returnvalue
    (`KismetSystemLibrary.PrintString` "OUCH")))

(fn `UserConstructionScript`)